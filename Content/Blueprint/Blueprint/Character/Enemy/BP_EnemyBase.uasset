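; Base enemy character Blueprint that handles health display, combat feedback and weapon attachment.
; BeginPlay creates the minion state widget, which Tick turns toward the camera and death hides.
; State and execution-stage events trigger parry and execution sounds, while action begin/end toggles an attached buff emitter during skill execution.
; The construction script snaps the weapon child actor to a mesh socket with an offset, and a helper event randomizes skeletal meshes.
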(event `self.ReceiveBeginPlay`
  ;[1 1 1] Begin Play
  (bind _returnvalue (`|CreateWidget` "/Game/Blueprint/Blueprint/Widget/W_MinionState.W_MinionState_C" null (`self.attributeComp`)))
  (`WidgetComponent.SetWidget` (`self.Health`) _returnvalue)
  (set `self.HealthWidget` _returnvalue)
  (add `self.OnStateChange` (delegate `OnStateChange_Event`))
  (add `self.OnExecuteStageChange` (delegate `OnExecuteStateChange_SFXIMPL`)))

(event `OnStateChange_Event` :!signature `self.OnStateChange`
  (params (state :type "ECharacterState Enum" :default "Idle"))
  ;[1 1 1] Begin Play
  (switch `ECharacterState` state
    (:`Stun`
      (`self.Play SFX` (`self.Parry AC`) "/Game/3rd_Party/ImportedSFX/DarkSouls/SC_Parry.SC_Parry"))
    (:`Death`
      (`SceneComponent.SetVisibility` (`self.Health`) false true)
      (`KismetSystemLibrary.PrintString` "die"))))

(event `OnExecuteStateChange_SFXIMPL` :!signature `self.OnExecuteStageChange`
  (params (ExecState :type "EExecutedState Enum" :default "NoExecuted"))
  ;[1 1 1] Begin Play
  (switch `EExecutedState` ExecState
    (:`ExecuteReaction`
      (`GameplayStatics.SpawnSoundAtLocation` "/Game/3rd_Party/ImportedSFX/DarkSouls/execute_Cue.execute_Cue" (`self.K2_GetActorLocation`) (struct) 1.0 1.0 0.0 null null))
    (:`Executed`
      (`GameplayStatics.SpawnSoundAtLocation` "/Game/3rd_Party/ImportedSFX/HitImpact/ExecutedBloodCue.ExecutedBloodCue" (`self.K2_GetActorLocation`) (struct) 1.0 1.0 0.0 null null))))

(event `RandomMeshGenerator`
  (params (`Mesh List` :type "Array of SkeletalMesh Object Reference") (Component :type "SkeletalMeshComponent Object Reference (by ref)"))
  ;[1 1 1] Randomize Mesh
  (set `SkeletalMeshComponent.SkeletalMeshAsset` (`|GetArrayItem` `Mesh List` (`KismetMathLibrary.RandomIntegerInRange` 0 (- (`KismetArrayLibrary.Array_Length` `Mesh List`) 1))) Component))

(event `self.ReceiveTick`
  (params (DeltaSeconds :type "Float (single-precision)"))
  (bind _returnvalue (`KismetMathLibrary.Normal` (- (`self.K2_GetActorLocation` (`GameplayStatics.GetPlayerCameraManager` 0)) (`self.K2_GetActorLocation`))))
  ;[1 1 1] Health Rotation
  (`SceneComponent.K2_SetWorldRotation` (`self.Health`) (`KismetMathLibrary.MakeRotator` 0.0 (`KismetMathLibrary.DegAtan2` (.z _returnvalue) (`KismetMathLibrary.VSizeXY` _returnvalue)) (`KismetMathLibrary.DegAtan2` (.y _returnvalue) (.x _returnvalue))) false false))

(event `EnableBuffVFX`
  ;[1 1 1] Buff Visibility Setup
  (if (`|EnumEquality` (`self.GetCharacterState`) "SkillExecuting")
    (`self.SpawnBuff`)
    (else
      (`self.DestroyBuff`))))

(event `self.actionComp.OnActionBegin`
  (params (OwnerCharacter :type "GodsArenaCharacter Object Reference") (CurrentAction :type "SAction Object Reference"))
  ;[1 1 1] Buff Visibility Setup
  (`self.EnableBuffVFX` :!label _label))

(event `self.actionComp.OnActionEnd`
  (params (OwnerCharacter :type "GodsArenaCharacter Object Reference") (CurrentAction :type "SAction Object Reference"))
  ;[1 1 1] Buff Visibility Setup
  (goto _label))

(fn `DestroyBuff`
  (bind _currentbuff (`self.CurrentBuff`))
  (`/Engine/EditorBlueprintResources/StandardMacros.IsValid` _currentbuff
    (:`Is Valid`
      (`ParticleSystemComponent.EndTrails` _currentbuff)
      (`ActorComponent.K2_DestroyComponent` _currentbuff))))

(fn `DestroySFX`
  (params (AudioComp :type "AudioComponent Object Reference (by ref)"))
  (`/Engine/EditorBlueprintResources/StandardMacros.IsValid` AudioComp
    (:`Is Valid`
      (`ActorComponent.K2_DestroyComponent` AudioComp))))

(fn `Play SFX`
  (params (AudioComp :type "AudioComponent Object Reference (by ref)") (Sound :type "SoundBase Object Reference") (AttenuationSettings :type "SoundAttenuation Object Reference"))
  (`self.DestroySFX` AudioComp)
  (bind _returnvalue (`GameplayStatics.SpawnSoundAtLocation` Sound (`self.K2_GetActorLocation`) (struct) 1.0 1.0 0.0 AttenuationSettings null))
  (`|VariableSetRef` AudioComp _returnvalue))

(fn `SpawnBuff`
  (bind _buffscale (`self.BuffScale`))
  (`/Engine/EditorBlueprintResources/StandardMacros.IsValid` (`self.CurrentBuff`)
    (:`Is Not Valid`
      (bind _returnvalue (`GameplayStatics.SpawnEmitterAttached` (`self.BuffTemplate`) (`self.BuffVFX`) "None" (0.0 0.0 0.0) (struct) (`KismetMathLibrary.MakeVector` _buffscale _buffscale _buffscale) "SnapToTarget" false))
      (set `self.CurrentBuff` _returnvalue))))

(fn `UserConstructionScript`
  (bind _childactor (`self.ChildActor`))
  (`SceneComponent.K2_AttachToComponent` _childactor (`self.Mesh`) (`self.WeaponSocket`) "SnapToTarget" "SnapToTarget" "KeepRelative" true)
  (`SceneComponent.K2_AddLocalTransform` _childactor (`self.AttachmentTransformOffset`) false false))