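; BP_ExpertKnight is a boss enemy character, the Knight, with modular armor randomized at spawn.
; The construction script makes the body follow the main mesh pose and the clothing pieces follow the body.
; On BeginPlay it picks random chest, shoulder, cloak and glove meshes from lists, then runs parent logic.
; It also shows a boss-state widget bound to its AttributeComp and registers itself with the player's TargetingComponent.
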(event `self.ReceiveBeginPlay`
  ;[1 1 1] Begin Play
  (`self.Cloth Generators`)
  (`parent.ReceiveBeginPlay`)
  (bind _returnvalue (`|CreateWidget` "/Game/Blueprint/Blueprint/Widget/W_BossState.W_BossState_C" (`GameplayStatics.GetPlayerController` 0)))
  (set `TextBlock.Text` "Knight" (`/Game/Blueprint/Blueprint/Widget/W_BossState.Name` _returnvalue))
  (set `/Game/Blueprint/Blueprint/Widget/W_BossState.Attribute Comp` (`self.attributeComp`) _returnvalue)
  (`UserWidget.AddToViewport` _returnvalue 0)
  (`TargetingComponent.AddTarget` (`self.GetComponentByClass` (`GameplayStatics.GetPlayerCharacter` 0) "/Script/GodArena_UE5.TargetingComponent") self))

(event `self.ReceiveTick`
  (params (DeltaSeconds :type "Float (single-precision)"))
  (`parent.ReceiveTick` DeltaSeconds))

(event `RandomMeshGenerator`
  (params (`Mesh List` :type "Array of SkeletalMesh Object Reference") (Component :type "SkeletalMeshComponent Object Reference (by ref)"))
  (set `SkeletalMeshComponent.SkeletalMeshAsset` (`|GetArrayItem` `Mesh List` (`KismetMathLibrary.RandomIntegerInRange` 0 (- (`KismetArrayLibrary.Array_Length` `Mesh List`) 1))) Component))

(event `Cloth Generators`
  (`self.RandomMeshGenerator` (`self.ChestList`) (`self.Chest`))
  (`self.RandomMeshGenerator` (`self.ShoulderList`) (`self.Shoulder`))
  (`self.RandomMeshGenerator` (`self.CloakList`) (`self.Cloak`))
  (`self.RandomMeshGenerator` (`self.GlovesList`) (`self.Gloves`)))

(fn `UserConstructionScript`
  (`parent.UserConstructionScript`)
  (`SkinnedMeshComponent.SetLeaderPoseComponent` (`self.RealBody`) (`self.Mesh`) true false)
  (`SkinnedMeshComponent.SetLeaderPoseComponent` (`self.Cloak`) (`self.RealBody`) false false)
  (`SkinnedMeshComponent.SetLeaderPoseComponent` (`self.Chest`) (`self.RealBody`) false false)
  (`SkinnedMeshComponent.SetLeaderPoseComponent` (`self.Shoulder`) (`self.RealBody`) false false)
  (`SkinnedMeshComponent.SetLeaderPoseComponent` (`self.Helmet`) (`self.RealBody`) false false)
  (`SkinnedMeshComponent.SetLeaderPoseComponent` (`self.Gloves`) (`self.RealBody`) false false)
  (`SkinnedMeshComponent.SetLeaderPoseComponent` (`self.Pant`) (`self.RealBody`) false false))