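; BP_TestDummy is an enemy test dummy with a state widget that faces the player's camera.
; On BeginPlay it creates a W_MinionState widget from its AttributeComp and assigns it to the Widget component.
; Each Tick billboards that component by computing world yaw and pitch toward the player camera with atan2, keeping roll at zero.
; It has no other active logic; a LaunchCharacter node is left unconnected.
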(event `self.ReceiveBeginPlay`
  (bind _returnvalue (`|CreateWidget` "/Game/Blueprint/Blueprint/Widget/W_MinionState.W_MinionState_C" null (`self.attributeComp`)))
  (`WidgetComponent.SetWidget` (`self.Widget`) _returnvalue))

(event `self.ReceiveTick`
  (params (DeltaSeconds :type "Float (single-precision)"))
  (bind _returnvalue (- (`self.K2_GetActorLocation` (`GameplayStatics.GetPlayerCameraManager` 0)) (`self.K2_GetActorLocation`)))
  (`SceneComponent.K2_SetWorldRotation` (`self.Widget`) (`KismetMathLibrary.MakeRotator` 0.0 (`KismetMathLibrary.DegAtan2` (.z _returnvalue) (`KismetMathLibrary.VSizeXY` _returnvalue)) (`KismetMathLibrary.DegAtan2` (.y _returnvalue) (.x _returnvalue))) false false))

(fn `UserConstructionScript`)