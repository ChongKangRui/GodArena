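; Expert Knight enemy character Blueprint with a randomized modular outfit and an overhead health widget.
; Construction links the body to the main mesh and the gear pieces to the body via leader pose.
; BeginPlay creates the minion state widget from the attribute component and randomizes chest, shoulder, cloak and glove meshes from lists.
; Tick rotates the health widget toward the player camera, and a state-change handler hides it on death.
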(event `self.ReceiveBeginPlay`
  ;[1 1 1] Begin Play
  (bind _returnvalue (`|CreateWidget` "/Game/Blueprint/Blueprint/Widget/W_MinionState.W_MinionState_C" null (`self.attributeComp`)))
  (`WidgetComponent.SetWidget` (`self.Health`) _returnvalue)
  (set `self.HealthWidget` _returnvalue)
  (`self.Cloth Generators`)
  (add `self.OnStateChange` (delegate `OnStateChange_Event`))
  (`KismetSystemLibrary.Delay` 1.0))

(event `OnStateChange_Event` :!signature `self.OnStateChange`
  (params (state :type "ECharacterState Enum" :default "Idle"))
  ;[1 1 1] Begin Play
  (if (`|EnumEquality` state "Death")
    (`SceneComponent.SetVisibility` (`self.Health`) false true)
    (`KismetSystemLibrary.PrintString` "die")))

(event `self.ReceiveTick`
  (params (DeltaSeconds :type "Float (single-precision)"))
  (bind _returnvalue (`KismetMathLibrary.Normal` (- (`self.K2_GetActorLocation` (`GameplayStatics.GetPlayerCameraManager` 0)) (`self.K2_GetActorLocation`))))
  (`SceneComponent.K2_SetWorldRotation` (`self.Health`) (`KismetMathLibrary.MakeRotator` 0.0 (`KismetMathLibrary.DegAtan2` (.z _returnvalue) (`KismetMathLibrary.VSizeXY` _returnvalue)) (`KismetMathLibrary.DegAtan2` (.y _returnvalue) (.x _returnvalue))) false false))

(event `RandomMeshGenerator`
  (params (`Mesh List` :type "Array of SkeletalMesh Object Reference") (Component :type "SkeletalMeshComponent Object Reference (by ref)"))
  (set `SkeletalMeshComponent.SkeletalMeshAsset` (`|GetArrayItem` `Mesh List` (`KismetMathLibrary.RandomIntegerInRange` 0 (- (`KismetArrayLibrary.Array_Length` `Mesh List`) 1))) Component))

(event `Cloth Generators`
  (`self.RandomMeshGenerator` (`self.ChestList`) (`self.Chest`))
  (`self.RandomMeshGenerator` (`self.ShoulderList`) (`self.Shoulder`))
  (`self.RandomMeshGenerator` (`self.CloakList`) (`self.Cloak`))
  (`self.RandomMeshGenerator` (`self.GlovesList`) (`self.Gloves`)))

(fn `UserConstructionScript`
  (`SkinnedMeshComponent.SetLeaderPoseComponent` (`self.RealBody`) (`self.Mesh`) true false)
  (`SkinnedMeshComponent.SetLeaderPoseComponent` (`self.Cloak`) (`self.RealBody`) false false)
  (`SkinnedMeshComponent.SetLeaderPoseComponent` (`self.Chest`) (`self.RealBody`) false false)
  (`SkinnedMeshComponent.SetLeaderPoseComponent` (`self.Shoulder`) (`self.RealBody`) false false)
  (`SkinnedMeshComponent.SetLeaderPoseComponent` (`self.Helmet`) (`self.RealBody`) false false)
  (`SkinnedMeshComponent.SetLeaderPoseComponent` (`self.Gloves`) (`self.RealBody`) false false)
  (`SkinnedMeshComponent.SetLeaderPoseComponent` (`self.Pant`) (`self.RealBody`) false false))