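; Samurai boss enemy that shows a named boss health widget and registers itself as a target with the player's targeting component.
; When damage leaves health at or below roughly 59%, it enters a second stage with an attack buff and hit reactions abandoned while attacking.
; That stage also permanently extends the weapon trace through its range-extend ability, enables the weapon trail and flags SecondStage on the AI Blackboard.
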(event `self.ReceiveBeginPlay`
  (`parent.ReceiveBeginPlay`)
  (bind _returnvalue (`|CreateWidget` "/Game/Blueprint/Blueprint/Widget/W_BossState.W_BossState_C" (`GameplayStatics.GetPlayerController` 0)))
  (set `TextBlock.Text` "Samurai" (`/Game/Blueprint/Blueprint/Widget/W_BossState.Name` _returnvalue))
  (set `/Game/Blueprint/Blueprint/Widget/W_BossState.Attribute Comp` (`self.attributeComp`) _returnvalue)
  (`UserWidget.AddToViewport` _returnvalue 0)
  (`TargetingComponent.AddTarget` (`self.GetComponentByClass` (`GameplayStatics.GetPlayerCharacter` 0) "/Script/GodArena_UE5.TargetingComponent") self)
  (`SceneComponent.K2_AttachToComponent` (`self.TargetingPointWidget`) (`self.Mesh`) "TargetPoint" "SnapToTarget" "KeepRelative" "KeepRelative" true))

(event `self.attributeComp.OnDamaged`
  (params (DamageCauser :type "Actor Object Reference") (Damage :type "Float (single-precision)") (debuff :type "AttackDebuff Structure"))
  (bind _attributecomp (`self.attributeComp`))
  (bind _weapon (`self.weapon`))
  (bind _blackboard (`AIController.Blackboard` (`AIBlueprintHelperLibrary.GetAIController` self)))
  (if (<= (`AttributeComponent.GetCurrentHealth` _attributecomp) (/ (`AttributeComponent.GetMaxHealth` _attributecomp) 1.7))
    (`self.SetCharacterBuff` (make `AttackBuff` :`NoParry` true))
    (`KismetArrayLibrary.Array_Add` (`AttributeComponent.HitReactionAbandonState` (`self.attributeComp`)) "Attacking")
    (bind _assaction_ability_ai_weapon_range_extend (cast `SAction_Ability_AI_WeaponRangeExtend` (`ActionComponent.GetAction` (`self.actionComp`) "SpecialAbility_01"))
      (:`then`
        (set `SAction_Ability_AI_WeaponRangeExtend.ForeverExtendWeapon` true _assaction_ability_ai_weapon_range_extend)
        (`BP_WeaponBase.ExtendTraceLength` _weapon (`SAction_Ability_AI_WeaponRangeExtend.ExtendedWeaponEndPosition` _assaction_ability_ai_weapon_range_extend))
        (set `BP_WeaponBase.TrailActivated` true _weapon)
        (`/Engine/EditorBlueprintResources/StandardMacros.IsValid` _blackboard
          (:`Is Valid`
            (`BlackboardComponent.SetValueAsBool` _blackboard "SecondStage" true))))
      (:`CastFailed`
        (`KismetSystemLibrary.PrintString` "cast failed?")))))

(fn `UserConstructionScript`
  (`parent.UserConstructionScript`))