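; Base bullet Blueprint that damages tagged actors overlapping its DamageCollision component.
; On an overlap with an actor carrying DamageActorTag, a DoOnce gate limits it to one hit, calling ApplyDamage with a random amount and debuff from WeaponAttribute.
; The hit also plays a 2D sword-hit sound.
; Debug prints report overlapped actors and damage results, including untagged overlaps.
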(event `self.ReceiveBeginPlay`
  (`parent.ReceiveBeginPlay`))

(event `self.DamageCollision.OnComponentBeginOverlap`
  (params (OverlappedComponent :type "PrimitiveComponent Object Reference") (OtherActor :type "Actor Object Reference") (OtherComp :type "PrimitiveComponent Object Reference") (OtherBodyIndex :type Integer) (bFromSweep :type Boolean) (SweepResult :type "HitResult Structure (by ref)"))
  (bind _returnvalue (`KismetSystemLibrary.GetDisplayName` OtherActor))
  (bind (_weaponattribute_attackanimation _weaponattribute_mindamage _weaponattribute_maxdamage _weaponattribute_cost _weaponattribute_attackdistance _weaponattribute_canparry _weaponattribute_debuff) (break `CharacterCombatAnimation` (`self.WeaponAttribute`)))
  (if (`self.ActorHasTag` OtherActor (`self.DamageActorTag`))
    (`KismetSystemLibrary.PrintString` _returnvalue)
    (`/Engine/EditorBlueprintResources/StandardMacros.DoOnce` false
      (:`Completed`
        (bind _returnvalue_2 (`GodArenaFunctionLibrary.ApplyDamage` self OtherActor (`KismetMathLibrary.RandomFloatInRange` _weaponattribute_mindamage _weaponattribute_maxdamage) _weaponattribute_debuff))
        (`KismetSystemLibrary.PrintString` (`KismetStringLibrary.Concat_StrStr` "Bullet/Buff attack success:" (`KismetStringLibrary.Conv_BoolToString` _returnvalue_2)))
        (`GameplayStatics.SpawnSound2D` "/Game/3rd_Party/ImportedSFX/HitImpact/SwordHit_Cue.SwordHit_Cue" 1.0 1.0 0.0 null)))
    (else
      (`KismetSystemLibrary.PrintString` _returnvalue true true (struct :`R` 1.0 :`G` 0.027019 :`A` 1.0) 10.0))))

(fn `UserConstructionScript`)