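; BP_kwangSkill_02 is a skill bullet actor, apparently Kwang's second skill, that deals a one-time area hit when spawned.
; BeginPlay speeds up its Niagara effect and runs a debug-drawn sphere trace for Pawns around its location.
; A DoOnce lets only the first hit actor with DamageActorTag take damage.
; That hit applies random damage and a debuff from WeaponAttribute, then prints the result.
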(event `self.ReceiveBeginPlay`
  (bind _returnvalue (`self.K2_GetActorLocation`))
  (bind (_weaponattribute_attackanimation _weaponattribute_mindamage _weaponattribute_maxdamage _weaponattribute_cost _weaponattribute_attackdistance _weaponattribute_canparry _weaponattribute_debuff) (break `CharacterCombatAnimation` (`self.WeaponAttribute`)))
  (`parent.ReceiveBeginPlay`)
  (`NiagaraComponent.SetCustomTimeDilation` (`self.NiagaraComponent`) 3.0)
  (bind _outhits (`KismetSystemLibrary.SphereTraceMultiForObjects` :`Start` _returnvalue :`End` (+ _returnvalue (0.0 0.0 1.0)) :`Radius` 300.0 :`ObjectTypes` (`|MakeArray` "ObjectTypeQuery3" :!type "EObjectTypeQuery Enum") :`DrawDebugType` "ForDuration"))
  (for _array_element _outhits
    (if (`self.ActorHasTag` (`.HitActor` (`GameplayStatics.BreakHitResult` _array_element)) (`self.DamageActorTag`))
      (`/Engine/EditorBlueprintResources/StandardMacros.DoOnce` false
        (:`Completed`
          (bind _returnvalue_2 (`GodArenaFunctionLibrary.ApplyDamage` self (`.HitActor` (`GameplayStatics.BreakHitResult` _array_element)) (`KismetMathLibrary.RandomFloatInRange` _weaponattribute_mindamage _weaponattribute_maxdamage) _weaponattribute_debuff))
          (`KismetSystemLibrary.PrintString` (`KismetStringLibrary.Concat_StrStr` "Bullet/Buff attack success:" (`KismetStringLibrary.Conv_BoolToString` _returnvalue_2))))))))

(fn `UserConstructionScript`
  (`parent.UserConstructionScript`))