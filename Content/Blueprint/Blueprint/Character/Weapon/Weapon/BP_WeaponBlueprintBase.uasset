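; Base weapon Blueprint that plays combat audio for swings, character effects and hit impacts.
; Binds to weapon trace events: trace begin plays swing and character sounds while the owner is Attacking.
; Trace hits pick a shield sound for Defending actors tagged CanShield, otherwise a weapon impact.
; SetSound rolls a percentage chance, destroys the previous audio component passed by reference and spawns a replacement attached to the mesh.
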(event `self.ReceiveBeginPlay`
  (`parent.ReceiveBeginPlay`)
  (add `self.OnWeaponBeginTrace` (delegate `OnWeaponBeginTrace_Event`))
  (add `self.OnWeaponTraceHit` (delegate `OnWeaponTraceHit_Event`)))

(event `OnWeaponTraceHit_Event` :!signature `self.OnWeaponTraceHit`
  (params (HitActor :type "GodsArenaCharacter Object Reference") (currentAttribute :type "CharacterCombatAnimation Structure"))
  (`/Engine/EditorBlueprintResources/StandardMacros.IsValid` HitActor
    (:`Is Valid`
      (if (and (`|EnumEquality` (`GodsArenaCharacter.GetCharacterState` HitActor) "Defending") (`self.ActorHasTag` HitActor "CanShield"))
        (`self.SetSound` (`self.ShieldHit`) (`self.HitImpactAC`))
        (else
          (`self.SetSound` (`self.WeaponHitImpact`) (`self.HitImpactAC`)))))))

(event `OnWeaponBeginTrace_Event`
  (bind _ownercharacter (`self.ownerCharacter`))
  (`/Engine/EditorBlueprintResources/StandardMacros.IsValid` _ownercharacter
    (:`Is Valid`
      (if (`|EnumEquality` (`GodsArenaCharacter.GetCharacterState` _ownercharacter) "Attacking")
        (`self.SetSound` (`self.SwingSound`) (`self.SwingAC`) "/Game/Blueprint/Blueprint/SFXSetting/ATT_WeaponSwing.ATT_WeaponSwing")
        (`self.SetSound` (`self.CharacterSFX`) (`self.CharacterSoundAC`) "/Game/Blueprint/Blueprint/SFXSetting/ATT_WeaponSwing.ATT_WeaponSwing" (`self.CharacterSFXTriggerChance`))))))

(fn `SetSound`
  (params (Sound :type "SoundBase Object Reference") (NewParam :type "AudioComponent Object Reference (by ref)") (AttenuationSettings :type "SoundAttenuation Object Reference") (PercentageToTrigger :type Integer :default 100))
  (bind _returnvalue (`KismetMathLibrary.RandomIntegerInRange` 1 100))
  (`KismetSystemLibrary.PrintString` (`KismetStringLibrary.Conv_IntToString` _returnvalue))
  (if (<= _returnvalue PercentageToTrigger)
    (`/Engine/EditorBlueprintResources/StandardMacros.IsValid` Sound
      (:`Is Valid`
        (`/Engine/EditorBlueprintResources/StandardMacros.IsValid` NewParam
          (:`Is Valid`
            (`ActorComponent.K2_DestroyComponent` NewParam))
          (:`Is Not Valid`
            _))
        (bind _returnvalue_2 (`GameplayStatics.SpawnSoundAttached` Sound (`self.mesh`) "None" (0.0 0.0 0.0) (struct) "KeepRelativeOffset" false 1.0 1.0 0.0 AttenuationSettings null))
        (`|VariableSetRef` NewParam _returnvalue_2))
      (:`Is Not Valid`
        (`KismetSystemLibrary.PrintString` "invalid sound effect")))))

(fn `UserConstructionScript`)