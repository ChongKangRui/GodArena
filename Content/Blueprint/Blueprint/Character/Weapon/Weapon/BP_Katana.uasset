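; BP_Katana is a katana weapon Blueprint that adds an optional trail to the weapon's tracing phase.
; It extends the parent's BeginTrace and EndTrace events, calling the parent first and then starting or ending the trail when TrailActivated is set.
; The construction script only calls the parent, and BeginPlay, overlap and Tick are unused.
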(event `self.BeginTrace`
  (`parent.BeginTrace`)
  (if (`self.TrailActivated`)
    (`self.BeginTrail`)))

(event `self.EndTrace`
  (`parent.EndTrace`)
  (if (`self.TrailActivated`)
    (`self.EndTrail`)))

(fn `UserConstructionScript`
  (`parent.UserConstructionScript`))