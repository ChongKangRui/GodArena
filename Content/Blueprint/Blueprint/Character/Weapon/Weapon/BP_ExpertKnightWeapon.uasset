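; Expert Knight weapon that adapts the parent weapon's hit tracing to the knight's current action.
; On BeginPlay it retries casting its owner until it gets the knight, then ends the weapon trail on state changes with no valid montage.
; Normal attacks use the parent trace, the first special lengthens it, and the second sphere-traces at the shield with its own radius.
; EndTrace also clears the shield trace timer and resets the radius.
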(event `self.ReceiveBeginPlay`
  (`parent.ReceiveBeginPlay`)
  (bind _asbp_expert_knight (cast `/Game/Blueprint/Blueprint/Character/Enemy/BP_ExpertKnight` (`self.ownerCharacter`) :!label _label)
    (:`then`
      (bind _output_get (set `self.As BP Expert Knight` _asbp_expert_knight))
      (add `GodsArenaCharacter.OnStateChange` _output_get (delegate `OnStateChange`)))
    (:`CastFailed`
      (`KismetSystemLibrary.Delay` 0.1)
      (goto _label))))

(event `OnStateChange`
  (params (state :type "ECharacterState Enum" :default "Idle"))
  (if (not (`KismetSystemLibrary.IsValid` (`Character.GetCurrentMontage` (`self.As BP Expert Knight`))))
    (`self.EndTrail`)))

(event `self.BeginTrace`
  (bind _as_bp_expert_knight (`self.As BP Expert Knight`))
  (bind _shieldtrace (`/Game/Blueprint/Blueprint/Character/Enemy/BP_ExpertKnight.ShieldTrace` _as_bp_expert_knight))
  (`/Engine/EditorBlueprintResources/StandardMacros.IsValid` _as_bp_expert_knight
    (:`Is Valid`
      (switch `ECombatType` (`ActionComponent.GetCurrentActionType` (`GodsArenaCharacter.actionComp` _as_bp_expert_knight))
        (:`NormalAttack`
          (`parent.BeginTrace`))
        (:`SpecialAbility_01`
          (`self.ExtendTraceLength` (`KismetMathLibrary.MakeVector` 0.0 0.0 20.0))
          (`parent.BeginTrace`))
        (:`SPecialAbility_02`
          (set `self.SphereRadius` (`self.Shiled Attack Sphere Radius`))
          (bind _returnvalue (`self.BeginTraceTick` _shieldtrace _shieldtrace "SphereTrace"))
          (set `self.Shield Trace Handle` _returnvalue))))))

(event `self.EndTrace`
  (`parent.EndTrace`)
  (`KismetSystemLibrary.K2_ClearAndInvalidateTimerHandle` (`self.Shield Trace Handle`))
  (set `self.SphereRadius` 20.0))

(fn `UserConstructionScript`
  (`parent.UserConstructionScript`))