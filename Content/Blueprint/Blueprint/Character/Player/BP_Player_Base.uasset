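; Base player character Blueprint that creates the state and tutorial widgets, handles the pause menu, and shows a death screen on death.
; An overlap sphere feeds enemies to TargetComponent for toggle and switch targeting, while dodge input runs through ActionComp.
; State and execution changes trigger sounds, with helpers that replace the previous audio component by reference.
; A timeline blends walk speed toward run speed and back.
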(event `OnExecuteStateChange` :!signature `self.OnExecuteStageChange`
  (params (ExecState :type "EExecutedState Enum" :default "NoExecuted"))
  (switch `EExecutedState` ExecState
    (:`ExecuteReaction`
      (`GameplayStatics.SpawnSoundAtLocation` null (`self.K2_GetActorLocation`) (struct) 1.0 1.0 0.0 null null))
    (:`Executed`
      (`GameplayStatics.SpawnSoundAtLocation` null (`self.K2_GetActorLocation`) (struct) 1.0 1.0 0.0 null null))))

(event `self.ReceiveBeginPlay`
  (add `self.OnStateChange` (delegate `OnStateChangeBind`))
  (bind _returnvalue (`|CreateWidget` "/Game/Blueprint/Blueprint/Widget/W_PlayerState.W_PlayerState_C" null (`self.attributeComp`)))
  (`UserWidget.AddToViewport` _returnvalue 0)
  (bind _returnvalue_2 (`|CreateWidget` (`self.TutorialWidgetClass`) (`GameplayStatics.GetPlayerController` 0)))
  (`UserWidget.AddToViewport` _returnvalue_2 0)
  (set `self.WBP_Tutorial` null)
  (add `self.OnExecuteStageChange` (delegate `OnExecuteStateChange`)))

(event `OnStateChangeBind` :!signature `self.OnStateChange`
  (params (state :type "ECharacterState Enum" :default "Idle"))
  (switch `ECharacterState` state
    (:`Stun`
      (`self.Play SFX` (`self.Stun AC`)))
    (:`Death`
      (`self.DeathModeActivated`))))

(event `DeathModeActivated`
  (bind _returnvalue (`GameplayStatics.GetPlayerController` 0))
  (bind _returnvalue_2 (`|CreateWidget` "/Game/Blueprint/Blueprint/Widget/W_DeadScene.W_DeadScene_C"))
  (`UserWidget.AddToViewport` _returnvalue_2 100)
  (set `PlayerController.bShowMouseCursor` true _returnvalue)
  (`WidgetBlueprintLibrary.SetInputMode_UIOnlyEx` _returnvalue _returnvalue_2))

(event `Key|RightMouseButton`
  (params (Key :type "Key Structure"))
  ;[1 0.03383 0] Example
)

(event `self.ReceiveTick`
  (params (DeltaSeconds :type "Float (single-precision)"))
  ;[1 0.03383 0] Example
)

(event `self.TargetedSphere.OnComponentBeginOverlap`
  (params (OverlappedComponent :type "PrimitiveComponent Object Reference") (OtherActor :type "Actor Object Reference") (OtherComp :type "PrimitiveComponent Object Reference") (OtherBodyIndex :type Integer) (bFromSweep :type Boolean) (SweepResult :type "HitResult Structure (by ref)"))
  ;[1 1 1] Target List
  (if (`self.ActorHasTag` OtherActor "Enemy")
    (bind _asgods_arena_character (cast `GodsArenaCharacter` OtherActor))
    (`TargetingComponent.AddTarget` (`self.TargetComponent`) _asgods_arena_character)))

(event `EnhancedInput|/Game/Blueprint/Blueprint/Character/EnhanceInput/InputAction/IA_SwitchTarget`
  (params (ActionValue :type "Float (double-precision)") (ElapsedSeconds :type "Float (double-precision)") (TriggeredSeconds :type "Float (double-precision)") (InputAction :type "InputAction Object Reference" :default "/Game/Blueprint/Blueprint/Character/EnhanceInput/InputAction/IA_SwitchTarget.IA_SwitchTarget"))
  (bind _targetcomponent (`self.TargetComponent`))
  ;[1 1 1] Switch Target
  (:`Started`
    (if (> ActionValue 0.0)
      (`TargetingComponent.SwitchTarget` _targetcomponent true)
      (else
        (`TargetingComponent.SwitchTarget` _targetcomponent false)))))

(event `self.TargetedSphere.OnComponentEndOverlap`
  (params (OverlappedComponent :type "PrimitiveComponent Object Reference") (OtherActor :type "Actor Object Reference") (OtherComp :type "PrimitiveComponent Object Reference") (OtherBodyIndex :type Integer))
  ;[1 1 1] Target List
  (bind _asgods_arena_character (cast `GodsArenaCharacter` OtherActor))
  (`TargetingComponent.RemoveTarget` (`self.TargetComponent`) _asgods_arena_character))

(event `EnhancedInput|/Game/Blueprint/Blueprint/Character/EnhanceInput/InputAction/IA_Target`
  (params (ActionValue :type Boolean) (ElapsedSeconds :type "Float (double-precision)") (TriggeredSeconds :type "Float (double-precision)") (InputAction :type "InputAction Object Reference" :default "/Game/Blueprint/Blueprint/Character/EnhanceInput/InputAction/IA_Target.IA_Target"))
  ;[1 1 1] Target
  (:`Started`
    (`TargetingComponent.ToggleTarget` (`self.TargetComponent`))))

(event `IncreaseSpeed`
  (bind _charactermovement (`self.CharacterMovement`))
  (bind _returnvalue (`MovementComponent.GetMaxSpeed` _charactermovement))
  ;[1 1 1] Set Speed
  (bind (_direction _newtrack_0) (`Timeline|SpeedIncrease` :!label _label)
    (:`Update`
      (switch `ETimelineDirection` _direction
        (:`Forward`
          (set `CharacterMovementComponent.MaxWalkSpeed` (`KismetMathLibrary.Lerp` _returnvalue (`self.Rnu Speed`) _newtrack_0) _charactermovement))
        (:`Backward`
          (set `CharacterMovementComponent.MaxWalkSpeed` (`KismetMathLibrary.Lerp` _returnvalue (`self.Walk Speed`) _newtrack_0) _charactermovement))))))

(event `EnhancedInput|/Game/Blueprint/Blueprint/Character/EnhanceInput/InputAction/IA_Dodge`
  (params (ActionValue :type Boolean) (ElapsedSeconds :type "Float (double-precision)") (TriggeredSeconds :type "Float (double-precision)") (InputAction :type "InputAction Object Reference" :default "/Game/Blueprint/Blueprint/Character/EnhanceInput/InputAction/IA_Dodge.IA_Dodge"))
  ;[1 1 1] Dodge
  (:`Started`
    (`ActionComponent.ExecuteAction` (`self.actionComp`) "Dodge")))

(event `DecreaseSpeed`
  ;[1 1 1] Set Speed
  (goto _label :!via `Reverse`))

(event `EnhancedInput|/Game/Blueprint/Blueprint/Character/EnhanceInput/InputAction/IA_PauseMenu`
  (params (ActionValue :type Boolean) (ElapsedSeconds :type "Float (double-precision)") (TriggeredSeconds :type "Float (double-precision)") (InputAction :type "InputAction Object Reference" :default "/Game/Blueprint/Blueprint/Character/EnhanceInput/InputAction/IA_PauseMenu.IA_PauseMenu"))
  ;[1 1 1] Pause Menu Setup
  (:`Started`
    (`self.Toggle Pause Menu`)))

(event `Toggle Pause Menu`
  (bind _returnvalue (`GameplayStatics.GetPlayerController` 0))
  (bind _returnvalue_2 (`GameplayStatics.GetPlayerController` 0))
  (bind _pausemenu (`self.PauseMenu`))
  ;[1 1 1] Pause Menu Setup
  (if (`|EnumInequality` (`self.GetCharacterState`) "Death")
    (`/Engine/EditorBlueprintResources/StandardMacros.IsValid` _pausemenu
      (:`Is Valid`
        (`Widget.RemoveFromParent` _pausemenu)
        (set `self.PauseMenu` null)
        (set `PlayerController.bShowMouseCursor` false _returnvalue)
        (`WidgetBlueprintLibrary.SetInputMode_GameOnly` _returnvalue)
        (`GameplayStatics.SetGamePaused` false))
      (:`Is Not Valid`
        (bind _returnvalue_3 (`|CreateWidget` "/Game/Blueprint/Blueprint/Widget/W_PauseMenu.W_PauseMenu_C" _returnvalue_2))
        (bind _output_get (set `self.PauseMenu` _returnvalue_3))
        (`GameplayStatics.SetGamePaused` true)
        (`UserWidget.AddToViewport` _output_get 100)
        (set `PlayerController.bShowMouseCursor` true _returnvalue_2)
        (`WidgetBlueprintLibrary.SetInputMode_GameAndUIEx` _returnvalue_2 _output_get)))
    (else
      (`KismetSystemLibrary.PrintString` "asdadasd"))))

(fn `DestroySFX`
  (params (AudioComp :type "AudioComponent Object Reference (by ref)"))
  (`/Engine/EditorBlueprintResources/StandardMacros.IsValid` AudioComp
    (:`Is Valid`
      (`ActorComponent.K2_DestroyComponent` AudioComp))))

(fn `Play SFX`
  (params (AudioComp :type "AudioComponent Object Reference (by ref)") (Sound :type "SoundBase Object Reference") (AttenuationSettings :type "SoundAttenuation Object Reference"))
  (`self.DestroySFX` AudioComp)
  (bind _returnvalue (`GameplayStatics.SpawnSoundAtLocation` Sound (`self.K2_GetActorLocation`) (struct) 1.0 1.0 0.0 AttenuationSettings null))
  (`|VariableSetRef` AudioComp _returnvalue))

(fn `PlaySoundWithChance`
  (params (Sound :type "SoundBase Object Reference") (NewParam :type "AudioComponent Object Reference (by ref)") (AttenuationSettings :type "SoundAttenuation Object Reference") (PercentageToTrigger :type Integer :default 100))
  (bind _returnvalue (`KismetMathLibrary.RandomIntegerInRange` 1 100))
  (`KismetSystemLibrary.PrintString` (`KismetStringLibrary.Conv_IntToString` _returnvalue))
  (if (<= _returnvalue PercentageToTrigger)
    (`/Engine/EditorBlueprintResources/StandardMacros.IsValid` Sound
      (:`Is Valid`
        (`/Engine/EditorBlueprintResources/StandardMacros.IsValid` NewParam
          (:`Is Valid`
            (`ActorComponent.K2_DestroyComponent` NewParam))
          (:`Is Not Valid`
            _))
        (bind _returnvalue_2 (`GameplayStatics.SpawnSoundAttached` Sound (`self.mesh`) "None" (0.0 0.0 0.0) (struct) "KeepRelativeOffset" false 1.0 1.0 0.0 AttenuationSettings null))
        (`|VariableSetRef` NewParam _returnvalue_2))
      (:`Is Not Valid`
        (`KismetSystemLibrary.PrintString` "invalid sound effect")))))

(fn `UserConstructionScript`)