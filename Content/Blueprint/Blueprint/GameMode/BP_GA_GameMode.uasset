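; BP_GA_GameMode is a game mode that spawns the player's pawn when play begins.
; BeginPlay switches to game-only input with a hidden cursor, then finds a PlayerStart actor.
; It spawns the Character class stored in BP_GameInstance at that location, keeping only its position, and has player controller 0 possess it.
; A missing start or failed cast prints a message.
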(event `self.ReceiveBeginPlay`
  (bind _returnvalue (`GameplayStatics.GetPlayerController` 0))
  (`WidgetBlueprintLibrary.SetInputMode_GameOnly` _returnvalue)
  (set `PlayerController.bShowMouseCursor` false _returnvalue)
  (bind _returnvalue_2 (`GameplayStatics.GetActorOfClass` "/Script/Engine.PlayerStart"))
  (`/Engine/EditorBlueprintResources/StandardMacros.IsValid` _returnvalue_2
    (:`Is Valid`
      (bind _asbp_game_instance (cast `/Game/Blueprint/Blueprint/BP_GameInstance` (`GameplayStatics.GetGameInstance`))
        (:`then`
          (bind _returnvalue_3 (`|SpawnActorFromClass` (`/Game/Blueprint/Blueprint/BP_GameInstance.character` _asbp_game_instance) (`KismetMathLibrary.Conv_VectorToTransform` (`self.K2_GetActorLocation` _returnvalue_2)) "Undefined" "OverrideRootScale" null null))
          (`Controller.Possess` (`GameplayStatics.GetPlayerController` 0) _returnvalue_3))
        (:`CastFailed`
          (`KismetSystemLibrary.PrintString` "Warning: BP_GameInstance Cast Failed"))))
    (:`Is Not Valid`
      (`KismetSystemLibrary.PrintString` "Error: No player start" true true (struct :`R` 1.0 :`G` 0.099472 :`A` 1.0) 6.0))))

(fn `UserConstructionScript`)